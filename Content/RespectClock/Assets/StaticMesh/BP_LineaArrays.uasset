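; BP_LineaArrays is a placement actor that lays out copies of a chosen static mesh in a straight-line array.
; The Construction Script loops over the count and adds local-space instances to an InstancedStaticMesh component, offsetting each by index times spacing along the Location vector.
; All instances share the same rotation and scale, and the Event Graph holds no runtime logic.
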(fn `UserConstructionScript`
  (for _index (range (`self.Count`))
    ;[1 1 1] メッシュの指定
    (`StaticMeshComponent.SetStaticMesh` (`self.InstancedStaticMesh`) (`self.New Mesh`))
    ;[1 1 1] 配置処理
    (`InstancedStaticMeshComponent.AddInstance` (`self.InstancedStaticMesh`) (`KismetMathLibrary.MakeTransform` (* (* _index (`self.Distance`)) (`self.Location`)) (`self.Rotation`) (`self.Scale`)) false)))