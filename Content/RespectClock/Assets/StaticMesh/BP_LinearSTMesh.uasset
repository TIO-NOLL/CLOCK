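; BP_LinearSTMesh is a procedural placement actor that lays out rows of repeated static meshes along straight lines.
; Its construction script creates one Instanced Static Mesh component per entry in LinearSTMeshInfoList.
; Each component then gets MeshCount local-space instances, stepped by Distance along the entry's X, Y or Z axis, with per-entry offset, rotation and scale.
; The event graph holds only empty placeholder events.
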(fn `UserConstructionScript`
  (for _array_element (`self.LinearSTMeshInfoList`)
    (bind _returnvalue (`AddComponent|NODE_AddInstancedStaticMeshComponent-0`))
    (`StaticMeshComponent.SetStaticMesh` _returnvalue (break `/Game/FLinearSTMeshInfo` _array_element))
    (`KismetArrayLibrary.Array_Add` (`self.Instanced STMesh List`) _returnvalue))
  (for (_array_element_2 _array_index) (`self.Instanced STMesh List`)
    (bind (_output_staticmesh _output_proctype _output_meshcount _output_offset _output_distance _output_meshrotation _output_meshscale) (break `/Game/FLinearSTMeshInfo` (`|GetArrayItem` (`self.LinearSTMeshInfoList`) _array_index)))
    (for _index (range _output_meshcount)
      (switch `/Game/EXYZType` _output_proctype
        (:`NewEnumerator0`
          (bind _returnvalue_2 (* _index _output_distance))
          (`InstancedStaticMeshComponent.AddInstance` _array_element_2 (`KismetMathLibrary.MakeTransform` (+ (`KismetMathLibrary.MakeVector` _returnvalue_2) _output_offset) _output_meshrotation _output_meshscale) false))
        (:`NewEnumerator1`
          (`InstancedStaticMeshComponent.AddInstance` _array_element_2 (`KismetMathLibrary.MakeTransform` (+ (`KismetMathLibrary.MakeVector` 0.0 _returnvalue_2) _output_offset) _output_meshrotation _output_meshscale) false))
        (:`NewEnumerator2`
          (`InstancedStaticMeshComponent.AddInstance` _array_element_2 (`KismetMathLibrary.MakeTransform` (+ (`KismetMathLibrary.MakeVector` 0.0 0.0 _returnvalue_2) _output_offset) _output_meshrotation _output_meshscale) false))))))