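; Player character Blueprint for RespectClock, handling the player's UI, screen effects and animation state.
; BeginPlay creates inventory and button-mash resist widgets, links anim class layers and caches ABP_Player.
; Inventory calls alternate between filling and opening the widget with look/move input locked, and closing it.
; Other events play game-mode fades, drive a vignette parameter collection from sanity, and toggle special animation, Jen visibility and an F5 fall flag.
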(event EventBPCallInventoryOpen
  (bind _returnvalue (Game|GetPlayerController 0))
  ;[1 1 1] インベントリ更新とインベントリを開く
  (Utilities|FlowControl|FlipFlop
    (:A
      (bind _returnvalue_2 (Class|Inventory|GetItem (Variables|Default|GetInventory)))
      (for (_array_element _array_index) _returnvalue_2
        (Default|AddSingleItemData (Variables|Default|GetInventoryWidget) (Variables|/Script/RespectClock.ItemBase|GetItemData _array_element) _array_index))
      (for _index (range (Utilities|Array|Length _returnvalue_2) 4)
        (Default|AddSingleItemData :self (Variables|Default|GetInventoryWidget) :SlotNum _index))
      (Input|SetIgnoreLookInput _returnvalue true)
      (Input|SetIgnoreMoveInput _returnvalue true)
      (Default|Open (Variables|Default|GetInventoryWidget)))
    (:B
      (Default|Close (Variables|Default|GetInventoryWidget))
      (Input|SetIgnoreLookInput _returnvalue false)
      (Input|SetIgnoreMoveInput _returnvalue false))))

(event EventBPCallUpdateInventory
  (params (_SlotNum :type Integer))
  ;[1 1 1] インベントリ更新とインベントリを開く
  (Default|ColorUpdate (Variables|Default|GetInventoryWidget) _SlotNum))

(event EventInFade
  (bind _asbpgm_respect_clock (Utilities|Casting|CastToBPGM_RespectClock (Game|GetGameMode)))
  (bind _userwidget (Default|FadeFunc _asbpgm_respect_clock "/Game/RespectClock/Core/Widget/GameOver/W_Fade.W_Fade_C"))
  (bind _asw_fade (Utilities|Casting|CastToW_Fade _userwidget))
  (Class|UserWidget|PlayAnimationForward _userwidget (Variables|/Game/RespectClock/Core/Widget/GameOver/W_Fade.W_Fade_C|GetFade _asw_fade) 1.0 false)
  (Utilities|FlowControl|Delay (Class|WidgetAnimation|GetEndTime (Variables|/Game/RespectClock/Core/Widget/GameOver/W_Fade.W_Fade_C|GetFade _asw_fade)))
  (Class|UserWidget|PlayAnimationReverse _userwidget (Variables|/Game/RespectClock/Core/Widget/GameOver/W_Fade.W_Fade_C|GetFade _asw_fade) 1.0 false))

(event EventUpdateVignette
  ;[1 1 1] パニックエフェクトの更新
  (if (> (Class|PlayerCharacter|GetSanity) 0.0)
    (Rendering|Material|SetScalarParameterValue "/Game/RespectClock/Effects/Vignette/MPC_Vignette.MPC_Vignette" "Power" (/ (Class|PlayerCharacter|GetSanity) 5.0) :!class /Script/Engine.KismetMaterialLibrary)))

(event EventSetAnimation
  ;[1 1 1] みなかったことにして
  (if (Variables|/Game/RespectClock/Characters/Player/Animation/ABP_CharacterBase.ABP_CharacterBase_C|GetIsSpecialAnim (Variables|Default|GetAnimBP))
    (Variables|/Game/RespectClock/Characters/Player/Animation/ABP_CharacterBase.ABP_CharacterBase_C|SetIsSpecialAnim (Variables|Default|GetAnimBP) false)
    (else
      (Variables|/Game/RespectClock/Characters/Player/Animation/ABP_CharacterBase.ABP_CharacterBase_C|SetIsSpecialAnim (Variables|Default|GetAnimBP) true))))

(event EventSetHidden
  (bind _jen (Variables|Default|GetJen))
  (if (Variables|/Script/Engine.SceneComponent|GetbVisible _jen)
    (Utilities|FlowControl|Delay 1.0)
    (Rendering|SetVisibility _jen false false)
    (else
      (Rendering|SetVisibility _jen true false))))

(event EventBeginPlay
  ;[1 1 1] 開始時にインベントリウィジェット作成
  (bind _returnvalue (UserInterface|CreateWidget "/Game/RespectClock/Core/Widget/Player/WBP_Inventory.WBP_Inventory_C"))
  (Variables|Default|SetInventoryWidget _returnvalue)
  (Components|SkeletalMesh|AnimationBlueprintLinking|LinkAnimClassLayers (Variables|Character|GetMesh) 0)
  (bind _asabp_player (Utilities|Casting|CastToABP_Player (Components|SkeletalMesh|GetAnimInstance (Variables|Character|GetMesh))))
  (Variables|Default|SetAnimBP _asabp_player)
  (bind _returnvalue_2 (UserInterface|CreateWidget "/Game/RespectClock/Core/Widget/Resist/WBP_ResistButton.WBP_ResistButton_C"))
  (bind _output_get (Variables|Default|SetResistedWidget _returnvalue_2))
  (UserInterface|Viewport|AddtoViewport _output_get 0)
  (Widget|SetVisibility (Variables|Default|GetResistedWidget) "Hidden"))

(event EventSetResistWidgetVisibility
  (params (_isibility :type Boolean))
  (bind _resistedwidget (Variables|Default|GetResistedWidget))
  ;[1 1 1] ボタン連打のＵＩ
  (if _isibility
    (Widget|SetVisibility _resistedwidget "Visible")
    (else
      (Widget|SetVisibility _resistedwidget "Hidden"))))

(event Input|KeyboardEvents|DebugKeyU
  (params (Key :type Key%20Structure :default "None") (ActionValue :type Input%20Action%20Value%20Structure)))

(event Input|KeyboardEvents|F5
  (params (Key :type Key%20Structure :default "None"))
  (:Pressed
    (if (Variables|Default|GetIsDoFall)
      (Variables|Default|SetIsDoFall false)
      (else
        (Variables|Default|SetIsDoFall true)))))

(fn ConstructionScript)