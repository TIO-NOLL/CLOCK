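; BP_RazorKiller is the RazorKiller character Blueprint, which forwards warp point and event calls to its AIC_RazorKiller AI controller.
; SetWarpPoint stores the given warp point and hands it to the controller through SetWarpPoints.
; Two debug custom events call the controller's StopEvent and SetEvent, the latter with a fixed value, to stop and start its event.
; The construction script, overlap and Tick are empty.
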(event `Debug_0`
  ;[1 1 0] StopEvent呼び出し用カスタムイベント（後で付ける）
  (bind _asaic_razor_killer (cast `AIC_RazorKiller` (`AIBlueprintHelperLibrary.GetAIController` self)))
  (`AIC_RazorKiller.StopEvent` _asaic_razor_killer))

(event `Debug_1`
  ;[1 1 0] StartEvent呼び出し用のカスタムイベント
  (bind _asaic_razor_killer (cast `AIC_RazorKiller` (`AIBlueprintHelperLibrary.GetAIController` self)))
  (`AIC_RazorKiller.SetEvent` _asaic_razor_killer 2.0))

(fn `SetWarpPoint`
  (params (WarpPoint :type "Array of /Game/RespectClock/Core/BP_WarpPoint Object Reference"))
  (bind _output_get (set `self.WarpPoint` WarpPoint))
  (bind _asaic_razor_killer (cast `AIC_RazorKiller` (`AIBlueprintHelperLibrary.GetAIController` self)))
  (`AIC_RazorKiller.SetWarpPoints` _asaic_razor_killer _output_get))

(fn `UserConstructionScript`)