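; One-shot trigger actor that ends the Razor Killer's active event when the player enters its box.
; It finds the killer's AI controller at BeginPlay, then on overlap adds a warp point ID key and stops that controller's event.
; It then fires ReActive, tells GM_RespectClock to end the track and destroys itself.
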(event `self.ReceiveBeginPlay`
  (bind _returnvalue (`GameplayStatics.GetActorOfClass` "/Script/RespectClock.AIC_RazorKiller"))
  (set `self.RazorKiller` _returnvalue))

(event `self.Box.OnComponentBeginOverlap`
  (params (OverlappedComponent :type "PrimitiveComponent Object Reference") (OtherActor :type "Actor Object Reference") (OtherComp :type "PrimitiveComponent Object Reference") (OtherBodyIndex :type Integer) (bFromSweep :type Boolean) (SweepResult :type "HitResult Structure (by ref)"))
  (bind _razorkiller (`self.RazorKiller`))
  (cast `PlayerCharacter` OtherActor)
  (`/Engine/EditorBlueprintResources/StandardMacros.DoOnce` false
    (:`Completed`
      (`AIC_RazorKiller.AddWarpPointIDKey` _razorkiller)
      (`AIC_RazorKiller.StopEvent` _razorkiller)
      (`self.ReActive`)
      (bind _asgm_respect_clock (cast `GM_RespectClock` (`GameplayStatics.GetGameMode`)))
      (`GM_RespectClock.EndTrack` _asgm_respect_clock)
      (`self.K2_DestroyActor`))))

(fn `UserConstructionScript`)