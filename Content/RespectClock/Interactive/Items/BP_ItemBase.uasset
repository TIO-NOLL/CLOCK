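; Base Blueprint for interactive items in RespectClock that highlight on overlap and can trigger game events.
; The construction script looks up a DataTable row by name and applies its mesh to the static mesh.
; Box overlap toggles an outline overlay material on that mesh.
; BPCallEventItem switches on EventData and plays the matching event, by ID or name, through the game instance's event player.
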(event `self.BPCallEventItem`
  (switch `EEventStatusItem` (`self.EventData`)
    (:`Killer`
      (bind _asrespect_clock_instance (cast `RespectClockInstance` (`GameplayStatics.GetGameInstance`)))
      (`EventPlayer.PlayEventByID` (`RespectClockInstance.GetEventPlayer` _asrespect_clock_instance) (`RespectClockInstance.GetWorldfromInstance` _asrespect_clock_instance) 6))
    (:`NASHI`
      (bind _asrespect_clock_instance_2 (cast `RespectClockInstance` (`GameplayStatics.GetGameInstance`)))
      (`EventPlayer.PlayEventByName` (`RespectClockInstance.GetEventPlayer` _asrespect_clock_instance_2) (`RespectClockInstance.GetWorldfromInstance` _asrespect_clock_instance_2) "お試し音再生"))))

(event `self.Box.OnComponentBeginOverlap`
  (params (OverlappedComponent :type "PrimitiveComponent Object Reference") (OtherActor :type "Actor Object Reference") (OtherComp :type "PrimitiveComponent Object Reference") (OtherBodyIndex :type Integer) (bFromSweep :type Boolean) (SweepResult :type "HitResult Structure (by ref)"))
  (`MeshComponent.SetOverlayMaterial` (`self.StaticMesh`) "/Game/RespectClock/Assets/Materials/M_Outline.M_Outline"))

(event `self.Box.OnComponentEndOverlap`
  (params (OverlappedComponent :type "PrimitiveComponent Object Reference") (OtherActor :type "Actor Object Reference") (OtherComp :type "PrimitiveComponent Object Reference") (OtherBodyIndex :type Integer))
  (`MeshComponent.SetOverlayMaterial` (`self.StaticMesh`) null))

(fn `UserConstructionScript`
  (bind _returnvalue (`|GetDataTableRow` (`self.DataTable`) (`self.RowName`))
    (:`then`
      (bind _output_get (set `self.ItemData` _returnvalue))
      (`StaticMeshComponent.SetStaticMesh` (`self.StaticMesh`) (`.Mesh` (break `ItemData` _output_get))))))