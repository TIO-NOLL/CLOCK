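; BP_Door is an interactive door object that exposes its RotationRoot through a getter; no rotation logic appears in this Blueprint.
; PlaySound plays the DoorOpen sound in 2D after a short delay.
; Leaving the Box trigger sets the M_Outline overlay on SMDoor, while entering does nothing.
; A disconnected chain that would apply the outline, cast to BP_RazorKiller and call Interactive never runs.
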(event `self.PlaySound`
  (`KismetSystemLibrary.Delay` 0.5)
  (`GameplayStatics.PlaySound2D` "/Game/RespectClock/Interactive/Audio/DoorOpen.DoorOpen" 1.0 1.0 0.0 null null))

(event `self.Box.OnComponentBeginOverlap`
  (params (OverlappedComponent :type "PrimitiveComponent Object Reference") (OtherActor :type "Actor Object Reference") (OtherComp :type "PrimitiveComponent Object Reference") (OtherBodyIndex :type Integer) (bFromSweep :type Boolean) (SweepResult :type "HitResult Structure (by ref)")))

(event `self.Box.OnComponentEndOverlap`
  (params (OverlappedComponent :type "PrimitiveComponent Object Reference") (OtherActor :type "Actor Object Reference") (OtherComp :type "PrimitiveComponent Object Reference") (OtherBodyIndex :type Integer))
  (`MeshComponent.SetOverlayMaterial` (`self.SM_Door`) "/Game/RespectClock/Assets/Materials/M_Outline.M_Outline"))

(fn `GetRotationRoot`
  (returns (ReturnValue :type "SceneComponent Object Reference"))
  (return (`self.RotationRoot`)))

(fn `UserConstructionScript`)