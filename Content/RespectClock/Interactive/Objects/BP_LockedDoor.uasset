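; BP_LockedDoor is an interactive locked door with messages for being locked, a wrong number and being unlocked.
; The Construction Script fills these message strings from DT_TextData through three chained row lookups by Japanese row names, each running only if the previous row is found.
; GetRotationRoot exposes the RotationRoot component, and the PlaySound event plays the DoorOpen sound in 2D after a short delay.
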(event `self.PlaySound`
  (`KismetSystemLibrary.Delay` 0.5)
  (`GameplayStatics.PlaySound2D` "/Game/RespectClock/Interactive/Audio/DoorOpen.DoorOpen" 1.0 1.0 0.0 null null))

(fn `GetRotationRoot`
  (returns (ReturnValue :type "SceneComponent Object Reference"))
  (return (`self.RotationRoot`)))

(fn `UserConstructionScript`
  (bind _returnvalue (`|GetDataTableRow` "/Game/RespectClock/Interactive/Items/DT_TextData.DT_TextData" "ドアロック")
    (:`then`
      (set `self.DisableMessage` (`KismetTextLibrary.Conv_TextToString` (break `TextData` _returnvalue)))
      (bind _returnvalue_2 (`|GetDataTableRow` "/Game/RespectClock/Interactive/Items/DT_TextData.DT_TextData" "番号違い")
        (:`then`
          (set `self.DifferentMessage` (`KismetTextLibrary.Conv_TextToString` (break `TextData` _returnvalue_2)))
          (bind _returnvalue_3 (`|GetDataTableRow` "/Game/RespectClock/Interactive/Items/DT_TextData.DT_TextData" "鍵開けた")
            (:`then`
              (set `self.OpenableMessage` (`KismetTextLibrary.Conv_TextToString` (break `TextData` _returnvalue_3))))))))))